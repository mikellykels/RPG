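; Trigger box actor that plays a flythrough Level Sequence cutscene once, on the first overlap.
; The sequence player is created at BeginPlay; overlap disables input, hides WBP_HUD and starts playback.
; A timer derived from the sequence's duration re-enables input on the overlapping actor and restores the HUD.
; The player-character check is unconnected, so the overlap is not filtered by actor.
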(event OnComponentBeginOverlap(Box)
  (params (OverlappedComponent :type Primitive%20Component%20Object%20Reference) (OtherActor :type Actor%20Object%20Reference) (OtherComp :type Primitive%20Component%20Object%20Reference) (OtherBodyIndex :type Integer) (bFromSweep :type Boolean) (SweepResult :type Hit%20Result%20Structure%20%28by%20ref%29))
  (bind _cutscene (Variables|Default|GetCutscene))
  (bind _returnvalue (Media|MediaPlayer|GetDuration _cutscene))
  (if true
    (Utilities|FlowControl|DoOnce false
      (:Completed
        (Variables|Default|SetOther%20Actor OtherActor)
        (Input|DisableInput 0)
        (bind _foundwidgets (Widget|GetAllWidgetsOfClass "/Game/RPG/Blueprints/UI/WBP_HUD.WBP_HUD_C" true))
        (for _array_element _foundwidgets
          (bind _output_get (Variables|Default|SetHUD _array_element))
          (Widget|SetVisibility _output_get "Hidden")
          (Sequencer|Player|Play _cutscene :!class /Script/MovieScene.MovieSceneSequencePlayer)
          (Utilities|Time|SetTimerbyEvent (delegate Custom|PlayerInputEnable) (/ (.value (.frame _returnvalue)) (.numerator (.framerate _returnvalue)))))))))

(event Custom|PlayerInputEnable
  (Input|EnableInput (Variables|Default|GetOther%20Actor) (Game|GetPlayerController 0))
  (Widget|SetVisibility (Variables|Default|GetHUD) "Visible"))

(event EventBeginPlay
  (bind _returnvalue (Sequencer|Player|CreateLevelSequencePlayer (Variables|Default|GetLevel%20Sequence)))
  (Variables|Default|SetCutscene _returnvalue))

(event Collision|EventActorBeginOverlap
  (params (OtherActor :type Actor%20Object%20Reference)))

(event EventTick
  (params (DeltaSeconds :type Float%20%28single-precision%29)))

(fn ConstructionScript)