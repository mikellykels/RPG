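; Attack system component that runs an axe melee combo by playing montages on CharacterMesh.
; TestAttack input, gated by CanAttack, starts an attack or buffers one in SaveAttack; AxeAttackCombo continues from that buffer or resets via StopCombo.
; AttackIndex chains montages B, A, then E, each behind a DoOnce and short delay.
; CharacterMesh setup is disconnected, and Attacks C and D sit outside the chain.
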(event Custom|AxeAttack
  ;[1 1 1] Axe Attack
  (if (Variables|Default|GetIsAttacking)
    (Variables|Default|SetSaveAttack true)
    (else
      (Variables|Default|SetIsAttacking true)
      (switch int (Variables|Default|GetAttackIndex)
        (:0
          (CallFunction|AttackB))
        (:1
          (CallFunction|AttackA))
        (:2
          (CallFunction|AttackE))))))

(event Custom|AxeAttackCombo
  ;[1 1 1] Combo continue
  (if (Variables|Default|GetSaveAttack)
    (Variables|Default|SetSaveAttack false)
    (switch int (Variables|Default|GetAttackIndex)
      (:0
        (CallFunction|AttackB))
      (:1
        (CallFunction|AttackA))
      (:2
        (CallFunction|AttackE)))
    (else
      (CallFunction|StopCombo))))

(event Custom|AttackC
  ;[1 1 1] Attack C
  (Utilities|FlowControl|DoOnce false :!label _label
    (:Completed
      (Utilities|FlowControl|Delay 0.1)
      (Animation|Montage|PlayMontage (Variables|Default|GetCharacterMesh) "/Game/SteamPunkCollection/SteamPunkAndroid/Animation/WeaponRightHand/Attack_C_Montage.Attack_C_Montage"
        (:then
          (Variables|Default|SetAttackIndex 2)
          (goto _label Reset))))))

(event Custom|AttackD
  ;[1 1 1] Attack D
  (Utilities|FlowControl|DoOnce false :!label _label
    (:Completed
      (Utilities|FlowControl|Delay 0.1)
      (Animation|Montage|PlayMontage (Variables|Default|GetCharacterMesh) "/Game/SteamPunkCollection/SteamPunkAndroid/Animation/WeaponRightHand/Attack_D_Montage.Attack_D_Montage"
        (:then
          (Variables|Default|SetAttackIndex 4)
          (goto _label Reset))))))

(event Custom|StopCombo
  ;[1 1 1] Stop combo
  (Variables|Default|SetIsAttacking false)
  (Variables|Default|SetAttackIndex 0))

(event Custom|AttackE
  ;[1 1 1] Attack E
  (Utilities|FlowControl|DoOnce false :!label _label
    (:Completed
      (Utilities|FlowControl|Delay 0.1)
      (Animation|Montage|PlayMontage (Variables|Default|GetCharacterMesh) "/Game/SteamPunkCollection/SteamPunkAndroid/Animation/WeaponRightHand/Attack_E_Montage.Attack_E_Montage"
        (:then
          (Variables|Default|SetAttackIndex 3)
          (goto _label Reset))))))

(event Custom|AttackA
  ;[1 1 1] Attack A
  (Utilities|FlowControl|DoOnce false :!label _label
    (:Completed
      (Utilities|FlowControl|Delay 0.1)
      (Animation|Montage|PlayMontage (Variables|Default|GetCharacterMesh) "/Game/SteamPunkCollection/SteamPunkAndroid/Animation/WeaponRightHand/Attack_A_Montage.Attack_A_Montage"
        (:then
          (Variables|Default|SetAttackIndex 2)
          (goto _label Reset))))))

(event Custom|AttackB
  ;[1 1 1] Attack B
  (Utilities|FlowControl|DoOnce false :!label _label
    (:Completed
      (Utilities|FlowControl|Delay 0.1)
      (Animation|Montage|PlayMontage (Variables|Default|GetCharacterMesh) "/Game/SteamPunkCollection/SteamPunkAndroid/Animation/WeaponRightHand/Attack_B_Montage.Attack_B_Montage"
        (:then
          (Variables|Default|SetAttackIndex 1)
          (goto _label Reset))))))

(event EventBeginPlay)

(event Input|ActionEvents|InputActionTestAttack
  (params (Key :type Key%20Structure :default "None"))
  ;[1 1 1] Attack input
  (:Pressed
    (if (Variables|Default|GetCanAttack)
      (CallFunction|AxeAttack))))