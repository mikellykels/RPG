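; Equipment component for an RPG character that stores weapons in a WeaponSlots array through AddWeapon.
; BeginPlay caches the owner's follow camera, which the TestInteract input uses for a debug-drawn forward sphere trace against WorldDynamic objects, though a hit triggers nothing.
; A debug H key prints each slot's row name.
; Logic for toggling the equipment widget with movement lock and for gathering item pickups is present but disconnected.
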(event EventBeginPlay
  (bind _asbp_rpgcharacter_base (Utilities|Casting|CastToBP_RPGCharacterBase (Components|GetOwner)))
  (Variables|Default|SetFollow%20Camera (Variables|/Game/RPG/Blueprints/Characters/BP_RPGCharacterBase.BP_RPGCharacterBase_C|GetFollowCamera _asbp_rpgcharacter_base)))

(event Input|ActionEvents|InputActionTestInteract
  (params (Key :type Key%20Structure :default "None"))
  (bind _follow_camera (Variables|Default|GetFollow%20Camera))
  (bind _returnvalue (Transformation|GetWorldLocation _follow_camera))
  (:Pressed
    (bind (_outhit _returnvalue_2) (Collision|SphereTraceForObjects _returnvalue (+ _returnvalue (* (Math|Vector|GetForwardVector (Transformation|GetWorldRotation _follow_camera)) "1000.000000,0.000000,0.000000")) 15.0 (Utilities|Array|MakeArray "ObjectTypeQuery2") false 0 "ForDuration"))
    (if _returnvalue_2
      _)))

(event Input|KeyboardEvents|DebugKeyH
  (params (Key :type Key%20Structure :default "None") (ActionValue :type Input%20Action%20Value%20Structure))
  (:Pressed
    (for _array_element (Variables|Default|GetWeaponSlots)
      (Development|PrintString (Utilities|String|ToString(Name) (.rowname (.item _array_element))) true true "(R=0.000000,G=0.660000,B=1.000000,A=1.000000)" 5.0))))

(event Input|KeyboardEvents|DebugKeyI
  (params (Key :type Key%20Structure :default "None") (ActionValue :type Input%20Action%20Value%20Structure)))

(fn AddWeapon
  (params (NewItem :type S%20Slots%20Structure%20%28by%20ref%29))
  (Utilities|Array|Add (Variables|Default|GetWeaponSlots) NewItem))