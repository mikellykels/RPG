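; Player stats component for the RPG, in which only experience and leveling logic is live.
; IncreaseXP adds XP and calls IncreaseLevel at the threshold, which raises the level, grows the XP requirement by a fixed step and resets XP to zero, discarding overflow.
; BeginPlay and the health and stamina functions are empty stubs; their old logic, owner detection and all HUD updates remain as disconnected nodes.
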(event EventBeginPlay)

(fn DecreaseHealth
  (params (Damage :type Float%20%28double-precision%29)))

(fn IncreaseMaxHealth
  (params (HealthIncremention :type Float%20%28double-precision%29)))

(fn DecreaseStamina
  (params (StaminaDepleted :type Float%20%28double-precision%29)))

(fn IncreaseMaxStamina
  (params (AddedStamina :type Float%20%28double-precision%29)))

(fn IncreaseHealth
  (params (AddedHealth :type Float%20%28double-precision%29)))

(fn IncreaseStamina
  (params (AddedStamina :type Float%20%28double-precision%29)))

(fn IncreaseXP
  (params (AddedXP :type Float%20%28double-precision%29))
  (Variables|XP|SetXP (+ (Variables|XP|GetXP) AddedXP))
  (if (>= (Variables|XP|GetXP) (Variables|XP|GetMaxXP))
    (LevelandXP|IncreaseLevel 1)))

(fn IncreaseLevel
  (params (AddedLevel :type Integer))
  (Variables|XP|SetLevel (+ (Variables|XP|GetLevel) AddedLevel))
  (Variables|XP|SetMaxXP (+ (Variables|XP|GetMaxXP) 1.5e+02))
  (Variables|XP|SetXP 0.0))